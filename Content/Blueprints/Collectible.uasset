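; Base collectible actor that drifts each tick by its speed times global time dilation unless paused, with an empty ApplyEffect hook.
; CheckCollisionType matches collider names, calling ApplyEffect for the player, then resets the collectible.
; Reset restores initial X and Y with a random height, and rerolls a random scale that also sets the collectible's value.
; Nothing in this graph calls the collision check, as its overlap event is disabled.
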(event `self.ReceiveTick`
  (params (DeltaSeconds :type "Float (single-precision)"))
  ;[1 1 1] Moving the collectible
  (if (not (`self.MovementPaused`))
    (`self.K2_AddActorWorldOffset` (* (`self.CollectibleSpeed`) (`GameplayStatics.GetGlobalTimeDilation`)))))

(fn `Apply Effect`)

(fn `CheckCollisionType`
  (params (`Actor Object Ref` :type "Actor Object Reference"))
  (locals (`Collider Object Name` :type String))
  (bind _output_get (set `local.Collider Object Name` (`KismetSystemLibrary.GetObjectName` `Actor Object Ref`)))
  (bind _collisionresult (`self.CheckForPlayerCollision` _output_get))
  (if _collisionresult
    (`self.Apply Effect`)
    (else
      (`self.CheckForRespawnCollision` (`local.Collider Object Name`))))
  (`self.ResetPosition`)
  (`self.ResetScaleAndValue`))

(fn `CheckForPlayerCollision`
  (params (ColliderObjectName :type String))
  (returns (CollisionResult :type Boolean))
  (return (`KismetStringLibrary.EqualEqual_StrStr` ColliderObjectName (`KismetSystemLibrary.GetObjectName` (`GameplayStatics.GetPlayerCharacter` 0)))))

(fn `CheckForRespawnCollision`
  (params (ColliderObjectName :type String))
  (returns (CollisionResult :type Boolean))
  (return (`KismetStringLibrary.EqualEqual_StrStr` ColliderObjectName (`self.RespawnTriggerName`))))

(fn `ResetPosition`
  (`self.K2_SetActorLocation` (`KismetMathLibrary.MakeVector` (.x (`self.CollectibleInitialPosition`)) (.y (`self.CollectibleInitialPosition`)) (`KismetMathLibrary.RandomFloatInRange` 50.0 400.0))))

(fn `ResetScaleAndValue`
  (bind _output_get (set `self.CollectibleScale` (`KismetMathLibrary.RandomFloatInRange` 1.0 5.0)))
  (bind _returnvalue (/ _output_get 2.0))
  (`self.SetActorScale3D` (`KismetMathLibrary.MakeVector` _returnvalue _returnvalue _returnvalue))
  (set `self.CollectibleValue` (`KismetMathLibrary.Round` (`self.CollectibleScale`))))

(fn `UserConstructionScript`)