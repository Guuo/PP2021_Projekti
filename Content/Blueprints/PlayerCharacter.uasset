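; Player character for a side-view game with flipbook sprites, a jump and a fuel-limited jetpack, locked against X-axis movement.
; Pressing jump while airborne starts a looping timer that drains fuel and launches upward below a speed cap, updating the InGameGUI fuel bar and Niagara exhaust.
; An animation state drives the sprite: negative Z velocity triggers Falling instead of apex notification, and hitting a "Surface"-tagged actor restores Idle and grounded state.
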(event `UpdateAnimation`
  ;[1 1 1] Handle animation changes
  (switch `/Game/Blueprints/PlayerAnimStates` (`self.AnimStates`)
    (:`NewEnumerator0`
      (`PaperFlipbookComponent.SetFlipbook` (`self.Sprite`) "/Game/Sprites/Idle.Idle")
      (`PaperFlipbookComponent.Play` (`self.Sprite`))
      (`PaperFlipbookComponent.SetLooping` (`self.Sprite`) true))
    (:`NewEnumerator1`
      (`PaperFlipbookComponent.SetFlipbook` (`self.Sprite`) "/Game/Sprites/Jump.Jump")
      (`PaperFlipbookComponent.Play` (`self.Sprite`))
      (`PaperFlipbookComponent.SetLooping` (`self.Sprite`) false))
    (:`NewEnumerator2`
      (`PaperFlipbookComponent.SetFlipbook` (`self.Sprite`) "/Game/Sprites/Falling.Falling")
      (`PaperFlipbookComponent.Play` (`self.Sprite`))
      (`PaperFlipbookComponent.SetLooping` (`self.Sprite`) false))))

(event `InputAction|Jump`
  (params (Key :type "Key Structure"))
  ;[1 1 1] Handle jump input
  (:`Pressed`
    (if (`self.IsAirborne`)
      (bind _returnvalue (`KismetSystemLibrary.K2_SetTimer` null "JetpackBoost" 0.016 true))
      (else
        (`self.Jump`)
        (set `self.AnimStates` "NewEnumerator1")
        (`self.UpdateAnimation`)
        (set `self.IsAirborne` true))))
  (:`Released`
    (`KismetSystemLibrary.K2_ClearAndInvalidateTimerHandle` _returnvalue)
    (`FXSystemComponent.SetFloatParameter` (`self.JetpackBoost_NS`) "User.BoostEffectSpawnRate" 0.0)))

(event `self.ReceiveBeginPlay`
  ;[1 1 1] Prevent movement along the X-axis, mainly in case of collisions moving the player
  (`MovementComponent.SetPlaneConstraintFromVectors` (`self.CharacterMovement`) (0.0 1.0 0.0) (0.0 0.0 1.0))
  (bind _foundwidgets (`WidgetBlueprintLibrary.GetAllWidgetsOfClass` "/Game/Blueprints/InGameGUI.InGameGUI_C"))
  (set `self.Found Widgets_0` _foundwidgets))

(event `self.ReceiveTick`
  (params (DeltaSeconds :type "Float (single-precision)"))
  ;[1 1 1] NotifyApex was finicky, using velocity check to trigger falling animation
  (if (< (.z (`MovementComponent.Velocity` (`self.CharacterMovement`))) 0.0)
    (`/Engine/EditorBlueprintResources/StandardMacros.DoOnce` false :!label _label
      (:`Completed`
        (set `self.AnimStates` "NewEnumerator2")
        (`self.UpdateAnimation`)
        (set `self.IsAirborne` true)))
    (else
      (goto _label :!via `Reset`))))

(event `self.CapsuleComponent.OnComponentHit`
  (params (HitComponent :type "PrimitiveComponent Object Reference") (OtherActor :type "Actor Object Reference") (OtherComp :type "PrimitiveComponent Object Reference") (NormalImpulse :type "Vector Structure") (Hit :type "HitResult Structure (by ref)"))
  ;[1 1 1] Handle animations when hitting a standable surface
  (`KismetSystemLibrary.PrintString` "Hello")
  (if (`self.ActorHasTag` OtherActor "Surface")
    (set `self.AnimStates` "NewEnumerator0")
    (`self.UpdateAnimation`)
    (set `self.IsAirborne` false)))

(fn `JetpackBoost`
  (locals (`Max Velocity` :type "Float (double-precision)" :default 1.57624))
  ;[1 1 1] Check fuel and decrement fuel if there is fuel left
  (if (> (`self.CurrentJetpackFuel`) 0.0)
    (set `self.CurrentJetpackFuel` (- (`self.CurrentJetpackFuel`) 0.1))
    ;[1 1 1] Clamp upwards velocity when using jetpack
    (if (> 300.0 (.z (`self.GetVelocity`)))
      (`self.LaunchCharacter` (0.0 0.0 20.0))
      (`/Game/Blueprints/InGameGUI.UpdateFuelBar` (`self.Found Widgets_0`) (`self.CurrentJetpackFuel`))
      (`FXSystemComponent.SetFloatParameter` (`self.JetpackBoost_NS`) "User.BoostEffectSpawnRate" 2000.0))
    (else
      (`FXSystemComponent.SetFloatParameter` (`self.JetpackBoost_NS`) "User.BoostEffectSpawnRate" 0.0))))

(fn `UserConstructionScript`)