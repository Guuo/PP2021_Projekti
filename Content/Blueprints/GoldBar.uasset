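; GoldBar is a spinning collectible that awards gold when the player touches it.
; On overlap it checks the other actor's object name, calling the gold-collected dispatcher with its value for the player, or running a respawn collision check otherwise.
; Both paths then reset its position, scale and value, so the actor is reused rather than destroyed.
; Tick calls the parent, then adds a per-frame rotation scaled by global time dilation, not delta time.
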(event `self.ReceiveActorBeginOverlap`
  (params (OtherActor :type "Actor Object Reference"))
  (bind _output_get (set `self.CollisionOtherActor` (`KismetSystemLibrary.GetObjectName` OtherActor)))
  (bind _collisionresult (`self.CheckForPlayerCollision` _output_get))
  (if _collisionresult
    (`self.GoldCollected_ED` (`self.CollectibleValue`))
    (else
      (`self.CheckForRespawnCollision` (`self.CollisionOtherActor`))))
  ;[1 1 1] Reset collectible state
  (`self.ResetPosition`)
  (`self.ResetScaleAndValue`))

(event `self.ReceiveTick`
  (params (DeltaSeconds :type "Float (single-precision)"))
  (`parent.ReceiveTick` 0.0)
  ;[1 1 1] Add rotation to collectible
  (`self.K2_AddActorWorldRotation` (* (`KismetMathLibrary.MakeRotator` 1.0 0.0 3.0) (`GameplayStatics.GetGlobalTimeDilation`))))

(fn `UserConstructionScript`)