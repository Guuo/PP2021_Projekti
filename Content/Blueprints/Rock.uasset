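; Rock is a physics-driven obstacle that launches on BeginPlay with a randomized sideways and upward impulse on its Sphere.
; On overlap, it fires the RockHitPlayer dispatcher for player hits or checks for respawn collision, then resets and relaunches.
; Resetting randomizes height and clears velocity to prevent momentum buildup.
; It builds on parent collision helpers, with ApplyEffect also firing the hit dispatcher.
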(event `self.ReceiveBeginPlay`
  (`parent.ReceiveBeginPlay`)
  (`self.LaunchObject`))

(event `self.ReceiveActorBeginOverlap`
  (params (OtherActor :type "Actor Object Reference"))
  (`self.CheckCollisionType` OtherActor)
  (bind _output_get (set `self.Collider Object Name_0` (`KismetSystemLibrary.GetObjectName` OtherActor)))
  (bind _collisionresult (`self.CheckForPlayerCollision` _output_get))
  (if _collisionresult
    ;[1 1 1] Rock hits player
    (`self.RockHitPlayer_ED`)
    (else
      (`self.CheckForRespawnCollision` (`self.Collider Object Name_0`))))
  ;[1 1 1] Rock hits respawn trigger, reset position
  (`self.ResetPosition`)
  (`self.ResetScaleAndValue`)
  (`self.LaunchObject`))

(fn `Apply Effect`
  (`parent.Apply Effect`)
  (`self.RockHitPlayer_ED`))

(fn `LaunchObject`
  (`PrimitiveComponent.AddImpulse` (`self.Sphere`) (`KismetMathLibrary.MakeVector` 0.0 (`KismetMathLibrary.RandomFloatInRange` -1000.0 -400.0) (`KismetMathLibrary.RandomFloatInRange` 200.0 700.0)) "None" true))

(fn `MoveAvoidableByTick`
  (`self.K2_AddActorWorldOffset` (* (`self.CollectibleSpeed`) (`GameplayStatics.GetGlobalTimeDilation`))))

(fn `ResetPosition`
  (`SceneComponent.K2_SetWorldTransform` (`self.Sphere`) (`KismetMathLibrary.Conv_VectorToTransform` (`KismetMathLibrary.MakeVector` (.x (`self.CollectibleInitialPosition`)) (.y (`self.CollectibleInitialPosition`)) (`KismetMathLibrary.RandomFloatInRange` 50.0 400.0))) false false)
  ;[1 1 1] Stop the rock from accumulating momentum on every position reset
  (`PrimitiveComponent.SetPhysicsLinearVelocity` (`self.Sphere`) (0.0 0.0 0.0) false "None"))

(fn `UserConstructionScript`
  (`parent.UserConstructionScript`))