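; Jetpack fuel pickup that spins in the world and grants fuel when the player collides with it.
; On overlap it checks the collider's name for the player and fires the jetpack-collected event dispatcher with its collectible value as fuel, otherwise running a respawn-collision check.
; After any overlap it resets position, scale and value, so the actor is recycled.
; Tick applies a rotation scaled by global time dilation.
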(event `self.ReceiveActorBeginOverlap`
  (params (OtherActor :type "Actor Object Reference"))
  (bind _output_get (set `self.ColliderName` (`KismetSystemLibrary.GetObjectName` OtherActor)))
  (bind _collisionresult (`self.CheckForPlayerCollision` _output_get))
  (if _collisionresult
    ;[1 1 1] Collectible value represents fuel
    (`self.JetpackCollected_ED` (`self.CollectibleValue`))
    (else
      (`self.CheckForRespawnCollision` (`self.ColliderName`))))
  ;[1 1 1] Reset collectible state
  (`self.ResetPosition`)
  (`self.ResetScaleAndValue`))

(event `self.ReceiveTick`
  (params (DeltaSeconds :type "Float (single-precision)"))
  (`parent.ReceiveTick` DeltaSeconds)
  ;[1 1 1] Add rotation to collectible
  (`self.K2_AddActorWorldRotation` (* (`KismetMathLibrary.MakeRotator` 1.0 0.0 3.0) (`GameplayStatics.GetGlobalTimeDilation`))))

(fn `UserConstructionScript`
  (`parent.UserConstructionScript`))